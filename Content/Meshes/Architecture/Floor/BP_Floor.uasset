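; BP_Floor is a floor piece with a ventilation grill that the player swings open and shut with E.
; Overlapping Box1 enables input and opens a gate, and leaving disables input and closes it.
; An integer toggle alternates between playing a timeline through the gate and reversing it directly, driving GrillMesh's roll.
; The construction script assigns a footstep-specific grill material to GrillMesh and GrillMesh2.
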(event `self.Box1.OnComponentBeginOverlap`
  (params (OtherActor :type "Actor Object Reference") (OtherComp :type "PrimitiveComponent Object Reference") (OtherBodyIndex :type Integer) (bFromSweep :type Boolean) (SweepResult :type "EngineTypes.HitResult Structure (by ref)"))
  (`self.EnableInput` (`GameplayStatics.GetPlayerController` 0))
  (goto _label :!via `Open`))

(event `self.Box1.OnComponentEndOverlap`
  (params (OtherActor :type "Actor Object Reference") (OtherComp :type "PrimitiveComponent Object Reference") (OtherBodyIndex :type Integer))
  (`|ExecutionSequence`
    (:`then_1`
      (`self.DisableInput` (`GameplayStatics.GetPlayerController` 0))
      (goto _label :!via `Close`))))

(event `Key|E`
  (:`Pressed`
    (switch `int` (`self.SwitchOnInt`)
      (:`0`
        (set `self.SwitchOnInt` 1)
        (`/Engine/EditorBlueprintResources/StandardMacros.Gate` true :!label _label
          (:`Exit`
            (bind (_direction _rotation) (`Timeline|Timeline_0` :!label _label_2)
              (:`Update`
                (`SceneComponent.K2_SetRelativeRotation` (`self.GrillMesh`) (`KismetMathLibrary.MakeRot` 0.0 0.0 (- 180.0 _rotation)) false))))))
      (:`1`
        (set `self.SwitchOnInt` 0)
        (goto _label_2 :!via `Reverse`)))))

(fn `UserConstructionScript`
  (`PrimitiveComponent.SetMaterial` (`self.GrillMesh2`) 0 "/Game/Meshes/Props/VentilationDucts/Gat_VentialtionGrill_Mat_ForFootsteps.Gat_VentialtionGrill_Mat_ForFootsteps")
  (`PrimitiveComponent.SetMaterial` (`self.GrillMesh`) 0 "/Game/Meshes/Props/VentilationDucts/Gat_VentialtionGrill_Mat_ForFootsteps.Gat_VentialtionGrill_Mat_ForFootsteps"))