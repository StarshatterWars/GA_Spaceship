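; Door frame Blueprint with two doors that slide open when something overlaps its trigger volume, provided ShouldBeOpen or ObjectiveCompleted is true.
; The DoorOpener timeline lerps both doors' relative locations from initial to end positions, and DoorCue plays alongside it.
; The end-overlap event only checks ShouldBeOpen and does nothing, so this graph never closes the doors.
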(event `self.TriggerVolume.OnComponentBeginOverlap`
  (params (OtherActor :type "Actor Object Reference") (OtherComp :type "PrimitiveComponent Object Reference") (OtherBodyIndex :type Integer) (bFromSweep :type Boolean) (SweepResult :type "EngineTypes.HitResult Structure (by ref)"))
  (if (`self.bShouldBeOpen`)
    (`|ExecutionSequence`
      (:`then_0`
        (bind (_direction _doordriver) (`Timeline|DoorOpener` :!label _label)
          (:`Update`
            (`|ExecutionSequence`
              (:`then_0`
                (`SceneComponent.K2_SetRelativeLocation` (`self.Door2`) (`KismetMathLibrary.VLerp` (`self.Door2InitLoc`) (`self.Door2EndLoc`) _doordriver) false))
              (:`then_1`
                (`SceneComponent.K2_SetRelativeLocation` (`self.Door1`) (`KismetMathLibrary.VLerp` (`self.DoorInitLoc`) (`self.DoorEndLoc`) _doordriver) false))))))
      (:`then_1`
        (`AudioComponent.Play` (`self.Door_Cue`) 0.0 :!label _label_2)))
    (elif (`self.bObjectiveCompleted`)
      (`|ExecutionSequence`
        (:`then_0`
          (goto _label))
        (:`then_1`
          (goto _label_2))))))

(event `self.TriggerVolume.OnComponentEndOverlap`
  (params (OtherActor :type "Actor Object Reference") (OtherComp :type "PrimitiveComponent Object Reference") (OtherBodyIndex :type Integer))
  (if (`self.bShouldBeOpen`)
    _))

(fn `UserConstructionScript`)