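; One-way elevator between a top and bottom floor, with timeline-driven sliding doors and sound.
; An overlap trigger opens the top doors once if ShouldBeOpen or CompletedObjective is set; AllowAccess sets the latter and re-arms it.
; A second trigger closes them and, after a delay, lerps each shell, door, frame and collision piece individually along one timeline.
; A destination trigger opens the bottom doors, which never close.
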(event `self.ReceiveBeginPlay`
  (`AudioComponent.SetSound` (`self.MovementSound`) (`self.MovingSound`))
  (`AudioComponent.SetSound` (`self.DoorSound`) (`self.DoorMoveSound`)))

(event `self.TriggerVolume.OnComponentBeginOverlap`
  (params (OverlappedComponent :type "PrimitiveComponent Object Reference") (OtherActor :type "Actor Object Reference") (OtherComp :type "PrimitiveComponent Object Reference") (OtherBodyIndex :type Integer) (bFromSweep :type Boolean) (SweepResult :type "HitResult Structure (by ref)"))
  (bind _doorsound (`self.DoorSound`))
  ;[1 1 1] Door Triggering
  (`/Engine/EditorBlueprintResources/StandardMacros.DoOnce` false :!label _label
    (:`Completed`
      (if (`self.bShouldBeOpen`)
        (`|ExecutionSequence` :!label _label_2
          (:`then_0`
            ;[1 1 1] Top Frame Door Movement
            (`AudioComponent.FadeIn` _doorsound 0.0 1.0 0.0)
            (bind (_direction _topdoordriver) (`Timeline|DoorOpener` :!label _label_3)
              (:`Update`
                (`|ExecutionSequence`
                  (:`then_0`
                    (`SceneComponent.K2_SetRelativeLocation` (`self.Door2`) (`KismetMathLibrary.VLerp` (`self.Door2InitLoc`) (`self.Door2EndLoc`) _topdoordriver) false false))
                  (:`then_1`
                    (`SceneComponent.K2_SetRelativeLocation` (`self.Door1`) (`KismetMathLibrary.VLerp` (`self.DoorInitLoc`) (`self.DoorEndLoc`) _topdoordriver) false false))))
              (:`Finished`
                (`AudioComponent.FadeOut` _doorsound 0.0 0.0))))
          (:`then_1`
            (`KismetSystemLibrary.Delay` 1.0)
            ;[1 1 1] Elevator Door Movement
            (bind (_direction_2 _elevatordoordriver) (`Timeline|ElevatorDoorOpener` :!label _label_4)
              (:`Update`
                (`|ExecutionSequence`
                  (:`then_0`
                    (`SceneComponent.K2_SetRelativeLocation` (`self.ElevatorDoor1`) (`KismetMathLibrary.VLerp` (`self.ElevatorDoor1InitLoc`) (`self.ElevatorDoor1EndLoc`) _elevatordoordriver) false false))
                  (:`then_1`
                    (`SceneComponent.K2_SetRelativeLocation` (`self.ElevatorDoor2`) (`KismetMathLibrary.VLerp` (`self.ElevatorDoor2InitLoc`) (`self.ElevatorDoor2EndLoc`) _elevatordoordriver) false false)))))))
        (elif (`self.CompletedObjective?`)
          (goto _label_2))))))

(event `self.TriggerVolElevatorMovement.OnComponentBeginOverlap`
  (params (OverlappedComponent :type "PrimitiveComponent Object Reference") (OtherActor :type "Actor Object Reference") (OtherComp :type "PrimitiveComponent Object Reference") (OtherBodyIndex :type Integer) (bFromSweep :type Boolean) (SweepResult :type "HitResult Structure (by ref)"))
  (bind _movementsound (`self.MovementSound`))
  ;[1 1 1] Elevator Shell Movement
  (`/Engine/EditorBlueprintResources/StandardMacros.DoOnce` false
    (:`Completed`
      (`|ExecutionSequence`
        (:`then_0`
          (`KismetSystemLibrary.Delay` 3.0)
          (`AudioComponent.FadeIn` _movementsound 0.0 1.0 0.0)
          (bind (_direction _elevatordriver) (`Timeline|ElevatorShellMovement`)
            (:`Update`
              (`|ExecutionSequence`
                (:`then_0`
                  (`SceneComponent.K2_SetRelativeLocation` (`self.ElevatorRightWall`) (`KismetMathLibrary.VLerp` (`self.ElevRightWallInitLoc`) (`self.ElevRightWallEndLoc`) _elevatordriver) false false))
                (:`then_1`
                  (`SceneComponent.K2_SetRelativeLocation` (`self.ElevatorLeftWall`) (`KismetMathLibrary.VLerp` (`self.ElevLeftWallInitLoc`) (`self.ElevLeftWallEndLoc`) _elevatordriver) false false))
                (:`then_2`
                  (`SceneComponent.K2_SetRelativeLocation` (`self.ElevatorBackWall`) (`KismetMathLibrary.VLerp` (`self.ElevBackWallInitLoc`) (`self.ElevBackWallEndLoc`) _elevatordriver) false false))
                (:`then_3`
                  (`SceneComponent.K2_SetRelativeLocation` (`self.ElevatorRoof`) (`KismetMathLibrary.VLerp` (`self.ElevRoofInitLoc`) (`self.ElevRoofEndLoc`) _elevatordriver) false false))
                (:`then_4`
                  (`SceneComponent.K2_SetRelativeLocation` (`self.ElevatorFloor`) (`KismetMathLibrary.VLerp` (`self.ElevFloorInitLoc`) (`self.ElevFloorEndLoc`) _elevatordriver) false false))
                (:`then_5`
                  (`SceneComponent.K2_SetRelativeLocation` (`self.ElevatorDoor2`) (`KismetMathLibrary.VLerp` (`self.ElevDoor2InitLoc`) (`self.ElevDoor2EndLoc`) _elevatordriver) false false))
                (:`then_6`
                  (`SceneComponent.K2_SetRelativeLocation` (`self.ElevatorDoor1`) (`KismetMathLibrary.VLerp` (`self.ElevDoor1InitLoc`) (`self.ElevDoor1EndLoc`) _elevatordriver) false false))
                (:`then_7`
                  (`SceneComponent.K2_SetRelativeLocation` (`self.ElevatorOutFrame`) (`KismetMathLibrary.VLerp` (`self.ElevOutFrameInitLoc`) (`self.ElevOutFrameEndLoc`) _elevatordriver) false false))
                (:`then_8`
                  (`SceneComponent.K2_SetRelativeLocation` (`self.ElevatorInFrame`) (`KismetMathLibrary.VLerp` (`self.ElevInFrameInitLoc`) (`self.ElevInFramEndLoc`) _elevatordriver) false false))
                (:`then_9`
                  (`SceneComponent.K2_SetRelativeLocation` (`self.ElevatorFrameRightCollision`) (`KismetMathLibrary.VLerp` (`self.ElevRightCollisionInitLoc`) (`self.ElevRightCollisionEndLoc`) _elevatordriver) false false))
                (:`then_10`
                  (`SceneComponent.K2_SetRelativeLocation` (`self.ElevatorFrameLeftCollision`) (`KismetMathLibrary.VLerp` (`self.ElevLeftCollisionInitLoc`) (`self.ElevLeftCollisionEndLoc`) _elevatordriver) false false))
                (:`then_11`
                  (`SceneComponent.K2_SetRelativeLocation` (`self.ElevatorFrameTopCollision`) (`KismetMathLibrary.VLerp` (`self.ElevTopCollisionInitLoc`) (`self.ElevTopCollisionEndLoc`) _elevatordriver) false false))))
            (:`Finished`
              (`AudioComponent.FadeOut` _movementsound 0.0 0.0))))
        (:`then_1`
          ;[1 1 1] Door Triggering
          (`|ExecutionSequence`
            (:`then_0`
              (`KismetSystemLibrary.Delay` 1.0)
              (goto _label_3 :!via `Reverse`))
            (:`then_1`
              (goto _label_4 :!via `Reverse`))))))))

(event `self.TriggerVolDesinationReached.OnComponentBeginOverlap`
  (params (OverlappedComponent :type "PrimitiveComponent Object Reference") (OtherActor :type "Actor Object Reference") (OtherComp :type "PrimitiveComponent Object Reference") (OtherBodyIndex :type Integer) (bFromSweep :type Boolean) (SweepResult :type "HitResult Structure (by ref)"))
  (bind _doorsound (`self.DoorSound`))
  ;[1 1 1] Door Triggering
  (`KismetSystemLibrary.Delay` 2.0)
  (`|ExecutionSequence`
    (:`then_0`
      (`KismetSystemLibrary.Delay` 1.0)
      ;[1 1 1] Bottom Frame Door Movement
      (`AudioComponent.FadeIn` _doorsound 0.0 1.0 0.0)
      (bind (_direction _bottomdoordriver) (`Timeline|BottomFrameDoors`)
        (:`Update`
          (`|ExecutionSequence`
            (:`then_0`
              (`SceneComponent.K2_SetRelativeLocation` (`self.BottomDoor2`) (`KismetMathLibrary.VLerp` (`self.BottomFloorDoor2InitLoc`) (`self.BottomFloorDoor2EndLoc`) _bottomdoordriver) false false))
            (:`then_1`
              (`SceneComponent.K2_SetRelativeLocation` (`self.BottomDoor1`) (`KismetMathLibrary.VLerp` (`self.BottomFloorDoor1InitLoc`) (`self.BottomFloorDoor1EndLoc`) _bottomdoordriver) false false))))
        (:`Finished`
          (`AudioComponent.FadeOut` _doorsound 0.0 0.0))))
    (:`then_1`
      ;[1 1 1] Elevator Door Movement
      (bind (_direction_2 _destreacheddoordriver) (`Timeline|DestinationReachedDoors`)
        (:`Update`
          (`|ExecutionSequence`
            (:`then_0`
              (`SceneComponent.K2_SetRelativeLocation` (`self.ElevatorDoor2`) (`KismetMathLibrary.VLerp` (`self.ElevDoor2EndLoc`) (`self.ElevDoor2EndOpenLoc`) _destreacheddoordriver) false false))
            (:`then_1`
              (`SceneComponent.K2_SetRelativeLocation` (`self.ElevatorDoor1`) (`KismetMathLibrary.VLerp` (`self.ElevDoor1EndLoc`) (`self.ElevDoor1EndOpenLoc`) _destreacheddoordriver) false false))))))))

(event `AllowAccess`
  ;[1 1 1] Door Triggering
  (set `self.CompletedObjective?` true)
  (goto _label :!via `Reset`))

(event `self.TriggerVolElevatorMovement.OnComponentEndOverlap`
  (params (OverlappedComponent :type "PrimitiveComponent Object Reference") (OtherActor :type "Actor Object Reference") (OtherComp :type "PrimitiveComponent Object Reference") (OtherBodyIndex :type Integer))
  ;[1 1 1] Elevator Shell Movement
)

(event `self.TriggerVolume.OnComponentEndOverlap`
  (params (OverlappedComponent :type "PrimitiveComponent Object Reference") (OtherActor :type "Actor Object Reference") (OtherComp :type "PrimitiveComponent Object Reference") (OtherBodyIndex :type Integer))
  ;[1 1 1] Door Triggering
)

(event `self.TriggerVolDesinationReached.OnComponentEndOverlap`
  (params (OverlappedComponent :type "PrimitiveComponent Object Reference") (OtherActor :type "Actor Object Reference") (OtherComp :type "PrimitiveComponent Object Reference") (OtherBodyIndex :type Integer))
  ;[1 1 1] Door Triggering
)

(fn `UserConstructionScript`)