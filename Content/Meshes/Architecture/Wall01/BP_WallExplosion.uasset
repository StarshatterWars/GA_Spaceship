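; Destructible wall actor that blows up when TriggerEventonActor fires, switching from intact to post-explosion mesh.
; The construction script shows PreExplosionWall01 with collision alongside PostExplosionWall02, hiding PostExplosionWall01 and the Explosion effect.
; The event plays Explosion twice a second apart, then a DoOnce swaps the Wall01 meshes and disables the intact wall's collision shortly after.
; The camera and controller-input functions are empty stubs returning defaults.
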(event `self.TriggerEventOnActor`
  ;[1 1 1] Triggers First Explosion And Second Explosion
  (`ActorComponent.Deactivate` (`self.Explosion`))
  (`SceneComponent.SetVisibility` (`self.Explosion`) true false)
  (`ActorComponent.Activate` (`self.Explosion`) false)
  (`KismetSystemLibrary.Delay` 1.0)
  (`ActorComponent.Deactivate` (`self.Explosion`))
  (`ActorComponent.Activate` (`self.Explosion`) false)
  ;[1 1 1] Switches Wall Meshes
  (`/Engine/EditorBlueprintResources/StandardMacros.DoOnce` false
    (:`Completed`
      (`SceneComponent.SetVisibility` (`self.PostExplosionWall_01`) true false)
      (`SceneComponent.SetVisibility` (`self.PreExplosionWall_01`) false false)
      ;[1 1 1] RemovesMeshCollision
      (`KismetSystemLibrary.Delay` 0.1)
      (`PrimitiveComponent.SetCollisionEnabled` (`self.PreExplosionWall_01`) "NoCollision"))))

(fn `GetCameraRotation`
  (returns (CameraRotation :type "Object.Rotator Structure"))
  (return))

(fn `RotateBackToCharacter`
  (params (CameraInitRotation :type "Object.Rotator Structure") (DeltaTime :type "Float (double-precision)") (InterpSpeed :type "Float (double-precision)"))
  (returns (NewParam :type Boolean))
  (return false))

(fn `RotateToTarget`
  (params (TargetLocation :type "Object.Vector Structure") (DeltaSeconds :type "Float (double-precision)") (InterpSpeed :type "Float (double-precision)") (StartRotation :type Boolean) (VectorOffset :type "Object.Vector Structure"))
  (returns (CameraEndLocation :type "Object.Rotator Structure"))
  (return))

(fn `SetControllerInput`
  (params (SetInput :type Boolean))
  (returns (NoOutput :type Boolean))
  (return false))

(fn `UserConstructionScript`
  (bind _preexplosionwall_01 (`self.PreExplosionWall_01`))
  (`SceneComponent.SetVisibility` _preexplosionwall_01 true false)
  (`SceneComponent.SetVisibility` (`self.PostExplosionWall_02`) true false)
  (`SceneComponent.SetVisibility` (`self.PostExplosionWall_01`) false false)
  (`SceneComponent.SetVisibility` (`self.Explosion`) false false)
  (`ActorComponent.Deactivate` (`self.Explosion`))
  (`PrimitiveComponent.SetCollisionEnabled` _preexplosionwall_01 "QueryAndPhysics"))