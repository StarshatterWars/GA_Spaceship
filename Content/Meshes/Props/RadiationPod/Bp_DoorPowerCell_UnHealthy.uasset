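; Unhealthy door power cell Blueprint, a radiation pod pickup that harms the player.
; Pickup trigger overlap applies damage to player 0, plays audio, then destroys the pod and trigger components.
; EnablePickup and DisablePickup open and close a gate whose exit leads to that same sequence.
; Geiger trigger overlaps toggle another gate when CanPodHurtPlayer is set, but nothing follows it, apparently a placeholder for audio.
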(event `self.PickupTrigger.OnComponentBeginOverlap`
  (params (OtherActor :type "Actor Object Reference") (OtherComp :type "PrimitiveComponent Object Reference") (OtherBodyIndex :type Integer) (bFromSweep :type Boolean) (SweepResult :type "EngineTypes.HitResult Structure (by ref)"))
  ;[1 1 1] Applys Damage To The Player and destroys actor
  (`GameplayStatics.ApplyDamage` (`GameplayStatics.GetPlayerCharacter` 0) 5.0 :!label _label)
  (`AudioComponent.Play` (`self.Audio1`) 0.0)
  (`ActorComponent.K2_DestroyComponent` (`self.RadiationPod`))
  (`ActorComponent.K2_DestroyComponent` (`self.PickupTrigger`)))

(event `self.GiegerTrigger.OnComponentBeginOverlap`
  (params (OtherActor :type "Actor Object Reference") (OtherComp :type "PrimitiveComponent Object Reference") (OtherBodyIndex :type Integer) (bFromSweep :type Boolean) (SweepResult :type "EngineTypes.HitResult Structure (by ref)"))
  ;[1 1 1] Could use something like this for audio implementation
  (if (`self.bCanPodHurtPlayer`)
    (`/Engine/EditorBlueprintResources/StandardMacros.Gate` true :!via `Open` :!label _label_2)))

(event `self.EnablePickup`
  (`/Engine/EditorBlueprintResources/StandardMacros.Gate` true :!via `Open` :!label _label_3
    (:`Exit`
      (goto _label))))

(event `self.GiegerTrigger.OnComponentEndOverlap`
  (params (OtherActor :type "Actor Object Reference") (OtherComp :type "PrimitiveComponent Object Reference") (OtherBodyIndex :type Integer))
  ;[1 1 1] Could use something like this for audio implementation
  (if (`self.bCanPodHurtPlayer`)
    (goto _label_2 :!via `Close`)))

(event `self.DisablePickup`
  (goto _label_3 :!via `Close`))

(fn `UserConstructionScript`)