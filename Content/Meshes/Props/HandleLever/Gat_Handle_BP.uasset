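; Interactable handle prop that rotates when the player interacts with it and notifies listeners through HandleInteract and HandleRelease dispatchers.
; A timeline drives the handle's relative roll forward on interact and reverses it on release or when an actor's overlap ends.
; Two DoOnce gates re-arm each other, so interact and release alternate and repeated calls are ignored.
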(event `self.OnInteract`
  ;[1 1 1] Animates The Handle When The Player Interacts With The Object
  (`/Engine/EditorBlueprintResources/StandardMacros.DoOnce` false :!label _label
    (:`Completed`
      (`|ExecutionSequence`
        (:`then_0`
          (bind (_direction _updaterot) (`Timeline|HAndleRot` :!label _label_2)
            (:`Update`
              (`SceneComponent.K2_SetRelativeRotation` (`self.Handle`) (`KismetMathLibrary.MakeRot` 0.0 0.0 _updaterot) false))))
        (:`then_1`
          (`self.HandleInteract`))
        (:`then_2`
          (goto _label_3 :!via `Reset`))))))

(event `self.OnRelease`
  ;[1 1 1] Animates The Handle When The Player Interacts With The Object
  (`/Engine/EditorBlueprintResources/StandardMacros.DoOnce` false :!label _label_3
    (:`Completed`
      (`|ExecutionSequence`
        (:`then_0`
          (goto _label_2 :!via `Reverse`))
        (:`then_1`
          (`self.HandleRelease`))
        (:`then_2`
          (goto _label :!via `Reset`))))))

(event `self.ReceiveActorEndOverlap`
  (params (OtherActor :type "Actor Object Reference"))
  ;[1 1 1] Animates The Handle When The Player Interacts With The Object
  (goto _label_3))

(fn `UserConstructionScript`)