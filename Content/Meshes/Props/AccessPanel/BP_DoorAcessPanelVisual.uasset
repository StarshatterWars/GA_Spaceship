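; Door access panel prop that fills its six holders with power cells when play begins.
; BeginPlay spawns a slightly scaled-down BP_DoorPowerCell at each holder mesh's socket.
; A Loop timeline holds logic to switch the panel to an access-granted material and unlock a chosen door or elevator once the objective completes.
; Nothing in this graph starts that timeline, so only the cell spawning runs.
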(event `self.ReceiveBeginPlay`
  (`|ExecutionSequence`
    (:`then_0`
      ;[1 1 1] Spawns A Power Cell On Each Clip
      (`|SpawnActorFromClass` "/Game/Meshes/Props/AccessPanel/BP_DoorPowerCell.BP_DoorPowerCell_C" (`KismetMathLibrary.MakeTransform` (.location (`SceneComponent.GetSocketTransform` (`self.Holder2`) "Socket" "RTS_World")) (.rotation (`SceneComponent.GetSocketTransform` (`self.Holder2`) "Socket" "RTS_World")) (0.95 0.95 0.95))))
    (:`then_1`
      (`|SpawnActorFromClass` "/Game/Meshes/Props/AccessPanel/BP_DoorPowerCell.BP_DoorPowerCell_C" (`KismetMathLibrary.MakeTransform` (.location (`SceneComponent.GetSocketTransform` (`self.Holder1`) "Socket" "RTS_World")) (.rotation (`SceneComponent.GetSocketTransform` (`self.Holder1`) "Socket" "RTS_World")) (0.95 0.95 0.95))))
    (:`then_2`
      (`|SpawnActorFromClass` "/Game/Meshes/Props/AccessPanel/BP_DoorPowerCell.BP_DoorPowerCell_C" (`KismetMathLibrary.MakeTransform` (.location (`SceneComponent.GetSocketTransform` (`self.Holder3`) "Socket" "RTS_World")) (.rotation (`SceneComponent.GetSocketTransform` (`self.Holder3`) "Socket" "RTS_World")) (0.95 0.95 0.95))))
    (:`then_3`
      (`|SpawnActorFromClass` "/Game/Meshes/Props/AccessPanel/BP_DoorPowerCell.BP_DoorPowerCell_C" (`KismetMathLibrary.MakeTransform` (.location (`SceneComponent.GetSocketTransform` (`self.Holder4`) "Socket" "RTS_World")) (.rotation (`SceneComponent.GetSocketTransform` (`self.Holder4`) "Socket" "RTS_World")) (0.95 0.95 0.95))))
    (:`then_4`
      (`|SpawnActorFromClass` "/Game/Meshes/Props/AccessPanel/BP_DoorPowerCell.BP_DoorPowerCell_C" (`KismetMathLibrary.MakeTransform` (.location (`SceneComponent.GetSocketTransform` (`self.Holder5`) "Socket" "RTS_World")) (.rotation (`SceneComponent.GetSocketTransform` (`self.Holder5`) "Socket" "RTS_World")) (0.95 0.95 0.95))))
    (:`then_5`
      (`|SpawnActorFromClass` "/Game/Meshes/Props/AccessPanel/BP_DoorPowerCell.BP_DoorPowerCell_C" (`KismetMathLibrary.MakeTransform` (.location (`SceneComponent.GetSocketTransform` (`self.Holder6`) "Socket" "RTS_World")) (.rotation (`SceneComponent.GetSocketTransform` (`self.Holder6`) "Socket" "RTS_World")) (0.95 0.95 0.95))))))

(fn `UserConstructionScript`)