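; BP_DoorPowerCell is an access-panel power cell prop that falls and bounces when DropCells is called.
; DropCells randomizes the projectile movement component's gravity scale and activates it, then a one-second delay loop destroys the actor after about six seconds, despite a comment saying ten.
; BeginPlay binds the projectile bounce event, which plays an explosion sound at the cell's location on each bounce.
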(event `self.DropCells`
  ;[1 1 1] Set Drop Speed
  (set `ProjectileMovementComponent.ProjectileGravityScale` (`KismetMathLibrary.RandomFloatInRange` 0.8 1.2) (`self.ProjectileMovement1`))
  ;[1 1 1] Gives Actor Physics
  (`ActorComponent.Activate` (`self.ProjectileMovement1`) false)
  ;[1 1 1] Destroys Actor 10 Seconds After Fail
  (set `self.Seconds` 0)
  (`KismetSystemLibrary.Delay` 1.0 :!label _label)
  (if (>= (`self.Seconds`) 5)
    (`self.K2_DestroyActor`)
    (else
      (`|ExecutionSequence`
        (:`then_0`
          (set `self.Seconds` (+ (`self.Seconds`) 1)))
        (:`then_1`
          (goto _label))))))

(event `self.ReceiveBeginPlay`
  ;[1 1 1] Place Audio Here For Canisters Bouncing SFX
  (add `ProjectileMovementComponent.OnProjectileBounce` (`self.ProjectileMovement1`) (delegate `OnProjectileBounce_Event`)))

(event `OnProjectileBounce_Event`
  (params (ImpactResult :type "EngineTypes.HitResult Structure (by ref)") (ImpactVelocity :type "Object.Vector Structure (by ref)"))
  ;[1 1 1] Place Audio Here For Canisters Bouncing SFX
  (`GameplayStatics.PlaySoundAtLocation` "/Game/Audio/SFX/Explosions/Explosion01.Explosion01" (`self.K2_GetActorLocation`)))

(fn `UserConstructionScript`)