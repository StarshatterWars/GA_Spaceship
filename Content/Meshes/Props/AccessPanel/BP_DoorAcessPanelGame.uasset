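; Door access panel running a timed objective: interacting starts a 60-second countdown to deliver power cells into six holders.
; Trigger overlaps feed DoN and MultiGate nodes that spawn socketed cells; the sixth completes the objective and lets KeycodeVolume start keycode entry.
; Timeout drops cells and resets through gates.
; Timelines for polling cell count and unlocking DoorToOpen after code entry have no visible start.
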(event `ObjectiveFailed`
  (bind _returnvalue (`GameplayStatics.GetPlayerCharacter` 0))
  ;[1 1 1] Animates The Button To Start The Objective
  (`|ExecutionSequence`
    (:`then_0`
      (bind (_direction _push) (`Timeline|ButtonMover` :!via `Reverse` :!label _label)
        (:`Update`
          (`SceneComponent.K2_SetRelativeLocation` (`self.Button`) (`KismetMathLibrary.MakeVector` (`KismetMathLibrary.Lerp` 21.0 17.0 _push)) false false)
          ;[1 1 1] Drop Off Control Logic
          (`/Engine/EditorBlueprintResources/StandardMacros.DoOnce` false :!label _label_2
            (:`Completed`
              ;[1 1 1] 60 Second Timer
              (set `self.Seconds` 60)
              (`KismetSystemLibrary.Delay` 1.0 :!label _label_3)
              (if (<= (`self.Seconds`) 0)
                (if (not (`self.ObjectiveComplete`))
                  (`|ExecutionSequence`
                    (:`then_0`
                      ;[1 1 1] Drops The Power Cells If The Player Is Not Quick Enough
                      (bind _outactors (`GameplayStatics.GetAllActorsOfClass` "/Game/Meshes/Props/AccessPanel/BP_DoorPowerCell.BP_DoorPowerCell_C"))
                      (message `/Game/PlayerController/DropPowerCellInterface.DropCells` _outactors))
                    (:`then_1`
                      ;[1 1 1] Fails The Objective
                      (`self.ObjectiveFailed`)
                      (bind _outactors_2 (`GameplayStatics.GetAllActorsOfClass` "/Game/Meshes/Props/RadiationPod/Bp_DoorPowerCell_UnHealthy.Bp_DoorPowerCell_UnHealthy_C"))
                      (message `/Game/PlayerController/PowerCellPickupInterface.StopDamage` _outactors_2)
                      ;[1 1 1] Resets The Objective
                      (`/Engine/EditorBlueprintResources/StandardMacros.IsValid` _returnvalue
                        (:`Is Valid`
                          (message `/Game/PlayerController/LevelResetInterface.Objective4Reset` _returnvalue)
                          (`self.ED_Objective4Reset`)
                          (`KismetSystemLibrary.Delay` 5.0)
                          (`|ExecutionSequence`
                            (:`then_0`
                              (goto _label_2 :!via `Reset`))
                            (:`then_1`
                              (goto _label_7 :!via `Reset`))
                            (:`then_2`
                              (goto _label_8 :!via `Reset`))
                            (:`then_3`
                              (goto _label_5 :!via `Open`))))))))
                (else
                  (`|ExecutionSequence`
                    (:`then_0`
                      (set `self.Seconds` (+ (`self.Seconds`) -1)))
                    (:`then_1`
                      (goto _label_3))))))))))
    (:`then_1`
      (goto _label_6 :!via `Close`))))

(event `/Game/PlayerController/OnEInteractInterface.OnInteract`
  ;[1 1 1] Animates The Button To Start The Objective
  (`/Engine/EditorBlueprintResources/StandardMacros.Gate` false :!label _label_4
    (:`Exit`
      (`/Engine/EditorBlueprintResources/StandardMacros.Gate` false :!label _label_5
        (:`Exit`
          (`|ExecutionSequence`
            (:`then_0`
              ;[1 1 1] Opens The HUD For This Objective
              (bind _outactors (`GameplayStatics.GetAllActorsOfClass` "/Game/PlayerController/Gat_PlayerHUD.Gat_PlayerHUD_C"))
              (for _array_element _outactors
                (bind _asgat_player_hud (cast `/Game/PlayerController/Gat_PlayerHUD` _array_element))
                (`/Game/PlayerController/Gat_PlayerHUD.ObjectiveOpen` _asgat_player_hud)))
            (:`then_1`
              (goto _label))
            (:`then_2`
              (goto _label_6 :!via `Open`))
            (:`then_3`
              (goto _label_5 :!via `Close`))
            (:`then_4`
              ;[1 1 1] Allows The Player To Pickup PowerCells
              (bind _outactors_2 (`GameplayStatics.GetAllActorsOfClass` "/Game/Meshes/Props/RadiationPod/BP_DoorPowerCell_Healthy.BP_DoorPowerCell_Healthy_C"))
              (message `/Game/PlayerController/PowerCellPickupInterface.EnablePickup` _outactors_2)
              ;[1 1 1] Allows Damage From Unhealthy Cells
              (bind _outactors_3 (`GameplayStatics.GetAllActorsOfClass` "/Game/Meshes/Props/RadiationPod/Bp_DoorPowerCell_UnHealthy.Bp_DoorPowerCell_UnHealthy_C"))
              (message `/Game/PlayerController/PowerCellPickupInterface.AllowPain` _outactors_3))))))))

(event `ObjectiveCompleted`
  ;[1 1 1] Animates The Button To Start The Objective
  (goto _label_4 :!via `Close`))

(event `self.Trigger.OnComponentBeginOverlap`
  (params (OverlappedComponent :type "PrimitiveComponent Object Reference") (OtherActor :type "Actor Object Reference") (OtherComp :type "PrimitiveComponent Object Reference") (OtherBodyIndex :type Integer) (bFromSweep :type Boolean) (SweepResult :type "HitResult Structure (by ref)"))
  ;[1 1 1] Drop Off Control Logic
  (`/Engine/EditorBlueprintResources/StandardMacros.Gate` true :!label _label_6
    (:`Exit`
      (if (> (`self.HowManyCells`) 0)
        (`/Engine/EditorBlueprintResources/StandardMacros.Do N` (`self.HowManyCells`) :!label _label_7
          (:`Exit`
            (`|MultiGate` false :!label _label_8
              (:`Out 0`
                ;[1 1 1] Spawns A Power Cell On Each Clip
                (`|SpawnActorFromClass` "/Game/Meshes/Props/AccessPanel/BP_DoorPowerCell.BP_DoorPowerCell_C" (`KismetMathLibrary.MakeTransform` (.location (`SceneComponent.GetSocketTransform` (`self.Holder2`) "Socket" "RTS_World")) (.rotation (`SceneComponent.GetSocketTransform` (`self.Holder2`) "Socket" "RTS_World")) (0.95 0.95 0.95)) "AlwaysSpawn" "OverrideRootScale")
                ;[1 1 1] Allows The Player TO Pick Up More Cells
                (bind _outactors (`GameplayStatics.GetAllActorsOfClass` "/Game/PlayerController/MyCharacter.MyCharacter_C" :!label _label_9))
                (message `/Game/PlayerController/PowerCellPickupInterface.ResetAmountOfPowerCells` _outactors)
                (`KismetSystemLibrary.Delay` 0.5)
                (`self.ResetDON`))
              (:`Out 1`
                (`|SpawnActorFromClass` "/Game/Meshes/Props/AccessPanel/BP_DoorPowerCell.BP_DoorPowerCell_C" (`KismetMathLibrary.MakeTransform` (.location (`SceneComponent.GetSocketTransform` (`self.Holder1`) "Socket" "RTS_World")) (.rotation (`SceneComponent.GetSocketTransform` (`self.Holder1`) "Socket" "RTS_World")) (0.95 0.95 0.95)) "AlwaysSpawn" "OverrideRootScale")
                (goto _label_9))
              (:`Out 2`
                (`|SpawnActorFromClass` "/Game/Meshes/Props/AccessPanel/BP_DoorPowerCell.BP_DoorPowerCell_C" (`KismetMathLibrary.MakeTransform` (.location (`SceneComponent.GetSocketTransform` (`self.Holder3`) "Socket" "RTS_World")) (.rotation (`SceneComponent.GetSocketTransform` (`self.Holder3`) "Socket" "RTS_World")) (0.95 0.95 0.95)) "AlwaysSpawn" "OverrideRootScale")
                (goto _label_9))
              (:`Out 3`
                (`|SpawnActorFromClass` "/Game/Meshes/Props/AccessPanel/BP_DoorPowerCell.BP_DoorPowerCell_C" (`KismetMathLibrary.MakeTransform` (.location (`SceneComponent.GetSocketTransform` (`self.Holder4`) "Socket" "RTS_World")) (.rotation (`SceneComponent.GetSocketTransform` (`self.Holder4`) "Socket" "RTS_World")) (0.95 0.95 0.95)) "AlwaysSpawn" "OverrideRootScale")
                (goto _label_9))
              (:`Out 4`
                (`|SpawnActorFromClass` "/Game/Meshes/Props/AccessPanel/BP_DoorPowerCell.BP_DoorPowerCell_C" (`KismetMathLibrary.MakeTransform` (.location (`SceneComponent.GetSocketTransform` (`self.Holder5`) "Socket" "RTS_World")) (.rotation (`SceneComponent.GetSocketTransform` (`self.Holder5`) "Socket" "RTS_World")) (0.95 0.95 0.95)) "AlwaysSpawn" "OverrideRootScale")
                (goto _label_9))
              (:`Out 5`
                (`|SpawnActorFromClass` "/Game/Meshes/Props/AccessPanel/BP_DoorPowerCell.BP_DoorPowerCell_C" (`KismetMathLibrary.MakeTransform` (.location (`SceneComponent.GetSocketTransform` (`self.Holder6`) "Socket" "RTS_World")) (.rotation (`SceneComponent.GetSocketTransform` (`self.Holder6`) "Socket" "RTS_World")) (0.95 0.95 0.95)) "AlwaysSpawn" "OverrideRootScale")
                ;[1 1 1] Checks There is enough time left and finishes the objective
                (if (> (`self.Seconds`) 0)
                  (set `self.Seconds` 0)
                  (set `self.ObjectiveComplete` true)
                  (`self.ObjectiveCompleted`)
                  ;[1 1 1] Disables The Pickup Of Healthy Cells
                  (bind _outactors_2 (`GameplayStatics.GetAllActorsOfClass` "/Game/Meshes/Props/RadiationPod/BP_DoorPowerCell_Healthy.BP_DoorPowerCell_Healthy_C"))
                  (message `/Game/PlayerController/PowerCellPickupInterface.DisablePickup` _outactors_2)
                  ;[1 1 1] Disables Damage From Unhealthy Cells
                  (bind _outactors_3 (`GameplayStatics.GetAllActorsOfClass` "/Game/Meshes/Props/RadiationPod/Bp_DoorPowerCell_UnHealthy.Bp_DoorPowerCell_UnHealthy_C"))
                  (message `/Game/PlayerController/PowerCellPickupInterface.StopDamage` _outactors_3)
                  (goto _label_10 :!via `Open`))))))))))

(event `ResetDON`
  ;[1 1 1] Drop Off Control Logic
  (goto _label_7 :!via `Reset`))

(event `self.KeycodeVolume.OnComponentBeginOverlap`
  (params (OverlappedComponent :type "PrimitiveComponent Object Reference") (OtherActor :type "Actor Object Reference") (OtherComp :type "PrimitiveComponent Object Reference") (OtherBodyIndex :type Integer) (bFromSweep :type Boolean) (SweepResult :type "HitResult Structure (by ref)"))
  (`/Engine/EditorBlueprintResources/StandardMacros.Gate` true :!label _label_10
    (:`Exit`
      (`/Engine/EditorBlueprintResources/StandardMacros.DoOnce` false
        (:`Completed`
          ;[1 1 1] Opens Key Code And Sets Code Version
          (bind _asmy_character (cast `/Game/PlayerController/MyCharacter` (`GameplayStatics.GetPlayerCharacter` 0)))
          (set `/Game/PlayerController/MyCharacter.bShouldBeKeyCodeVersion1` true _asmy_character)
          (`/Game/PlayerController/MyCharacter.EnterKeyCodeSequence` _asmy_character))))))

(fn `GetSecondsLeft`
  (returns (`Seconds Left` :type Integer))
  (return (`self.Seconds`)))

(fn `UserConstructionScript`)