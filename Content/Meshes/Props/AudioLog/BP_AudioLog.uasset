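; BP_AudioLog is a collectible audio log prop that the player picks up with the E key.
; Overlapping PickupVolume shows a HUD message, enables input and opens a gate; leaving sends the exit message, disables input and closes it.
; Pressing E through the open gate hides the log, marks the AccessPanel objective completed, calls LogCollected and destroys the actor.
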(event `self.PickupVolume.OnComponentBeginOverlap`
  (params (OtherActor :type "Actor Object Reference") (OtherComp :type "PrimitiveComponent Object Reference") (OtherBodyIndex :type Integer) (bFromSweep :type Boolean) (SweepResult :type "EngineTypes.HitResult Structure (by ref)"))
  (bind _outactors (`GameplayStatics.GetAllActorsOfClass` "/Game/PlayerController/Gat_PlayerHUD.Gat_PlayerHUD_C"))
  (message `/Game/Meshes/Props/Pipes/BPI_PipeInterface.Pipe To HUD In Volume` _outactors)
  (`self.EnableInput` (`GameplayStatics.GetPlayerController` 0))
  (goto _label :!via `Open`))

(event `self.PickupVolume.OnComponentEndOverlap`
  (params (OtherActor :type "Actor Object Reference") (OtherComp :type "PrimitiveComponent Object Reference") (OtherBodyIndex :type Integer))
  (bind _outactors (`GameplayStatics.GetAllActorsOfClass` "/Game/PlayerController/Gat_PlayerHUD.Gat_PlayerHUD_C"))
  (message `/Game/Meshes/Props/Pipes/BPI_PipeInterface.PipeToHudOutVolume` _outactors)
  (`self.DisableInput` (`GameplayStatics.GetPlayerController` 0))
  (goto _label :!via `Close`))

(event `Key|E`
  (:`Pressed`
    (`|ExecutionSequence`
      (:`then_0`
        (`/Engine/EditorBlueprintResources/StandardMacros.Gate` true :!label _label
          (:`Exit`
            (`SceneComponent.SetVisibility` (`self.AudioLog`) false false)
            (set `/Game/Meshes/Props/AccessPanel/BP_DoorAcessPanelVisual.bObjectiveCompleted` true (`self.AccessPanel`))
            (`self.LogCollected`)
            (`self.K2_DestroyActor`)))))))

(fn `UserConstructionScript`)