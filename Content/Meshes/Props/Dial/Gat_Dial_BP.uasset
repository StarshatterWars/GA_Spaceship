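; Interactable dial prop that rotates while the player interacts with it and turns back when released.
; Interacting plays the DialRotate timeline to drive the dial mesh's pitch and calls DialInteract.
; Release or an actor ending overlap reverses the timeline and calls DialRelease.
; Two DoOnce gates re-arm each other, so interact and release alternate without repeat triggers.
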(event `self.OnInteract`
  ;[1 1 1] Animates The Dial To Rotate When The Player Interacts With The Object
  (`/Engine/EditorBlueprintResources/StandardMacros.DoOnce` false :!label _label
    (:`Completed`
      (`|ExecutionSequence`
        (:`then_0`
          (bind (_direction _newtrack_0) (`Timeline|DialRotate` :!label _label_2)
            (:`Update`
              (`SceneComponent.K2_SetRelativeRotation` (`self.Dial`) (`KismetMathLibrary.MakeRot` _newtrack_0 90.0 90.0) false))))
        (:`then_1`
          (`self.DialInteract`))
        (:`then_2`
          (goto _label_3 :!via `Reset`))))))

(event `self.OnRelease`
  ;[1 1 1] Animates The Dial To Rotate When The Player Interacts With The Object
  (`/Engine/EditorBlueprintResources/StandardMacros.DoOnce` false :!label _label_3
    (:`Completed`
      (`|ExecutionSequence`
        (:`then_0`
          (goto _label_2 :!via `Reverse`))
        (:`then_1`
          (`self.DialRelease`))
        (:`then_2`
          (goto _label :!via `Reset`))))))

(event `self.ReceiveActorEndOverlap`
  (params (OtherActor :type "Actor Object Reference"))
  ;[1 1 1] Animates The Dial To Rotate When The Player Interacts With The Object
  (goto _label_3))

(fn `UserConstructionScript`)