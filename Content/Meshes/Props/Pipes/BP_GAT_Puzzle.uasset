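; Pipe repair puzzle where the player fits three collected pickups (curve, X and T sections) into gaps in the pipework.
; Each trigger checks its pickup, messages the HUD and enables input, so pressing E reveals that section and stops its randomly scaled particles.
; Gates scope E to the active trigger and lock finished sections.
; A shared MultiGate fades one audio per repair, flagging the AccessPanel objective complete on the third.
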(event `self.ReceiveBeginPlay`
  (bind _returnvalue (`KismetMathLibrary.MakeVector` (`KismetMathLibrary.RandomFloatInRange` 0.5 1.5) (`KismetMathLibrary.RandomFloatInRange` 0.5 1.5) (`KismetMathLibrary.RandomFloatInRange` 0.5 1.5)))
  ;[1 1 1] Randomly Sets The Scale For The Particles
  (`SceneComponent.SetRelativeScale3D` (`self.ParticleSystem7`) _returnvalue)
  (`SceneComponent.SetRelativeScale3D` (`self.ParticleSystem6`) _returnvalue)
  (`SceneComponent.SetRelativeScale3D` (`self.ParticleSystem5`) _returnvalue)
  (`SceneComponent.SetRelativeScale3D` (`self.ParticleSystem4`) _returnvalue)
  (`SceneComponent.SetRelativeScale3D` (`self.ParticleSystem3`) _returnvalue)
  (`SceneComponent.SetRelativeScale3D` (`self.ParticleSystem2`) _returnvalue)
  (`SceneComponent.SetRelativeScale3D` (`self.ParticleSystem1`) _returnvalue))

(event `self.CurveSectionTrigger.OnComponentBeginOverlap`
  (params (OtherActor :type "Actor Object Reference") (OtherComp :type "PrimitiveComponent Object Reference") (OtherBodyIndex :type Integer) (bFromSweep :type Boolean) (SweepResult :type "EngineTypes.HitResult Structure (by ref)"))
  (bind _returnvalue (`GameplayStatics.GetPlayerController` 0))
  ;[1 1 1] Handles All The Input For The Curved Pipe Section
  (if (`/Game/Meshes/Props/Pipes/BP_GAT_Pipe_CurveSection.bCollected` (`self.PickupCurveSection`))
    (`/Engine/EditorBlueprintResources/StandardMacros.Gate` false :!label _label
      (:`Exit`
        (bind _outactors (`GameplayStatics.GetAllActorsOfClass` "/Game/PlayerController/Gat_PlayerHUD.Gat_PlayerHUD_C"))
        (message `/Game/Meshes/Props/Pipes/BPI_PipeInterface.Pipe To HUD In Volume` _outactors)
        (`self.EnableInput` _returnvalue)
        (goto _label_3 :!via `Open`)))))

(event `self.CurveSectionTrigger.OnComponentEndOverlap`
  (params (OtherActor :type "Actor Object Reference") (OtherComp :type "PrimitiveComponent Object Reference") (OtherBodyIndex :type Integer))
  ;[1 1 1] Handles All The Input For The Curved Pipe Section
  (bind _outactors (`GameplayStatics.GetAllActorsOfClass` "/Game/PlayerController/Gat_PlayerHUD.Gat_PlayerHUD_C" :!label _label_2))
  (message `/Game/Meshes/Props/Pipes/BPI_PipeInterface.PipeToHudOutVolume` _outactors)
  (`self.DisableInput` (`GameplayStatics.GetPlayerController` 0))
  (goto _label_3 :!via `Close`))

(event `Key|E`
  (bind _returnvalue (`GameplayStatics.GetPlayerController` 0))
  (bind _returnvalue_2 (`GameplayStatics.GetPlayerController` 0))
  (:`Pressed`
    (`|ExecutionSequence`
      (:`then_0`
        ;[1 1 1] Handles All The Input For The Curved Pipe Section
        (`/Engine/EditorBlueprintResources/StandardMacros.Gate` true :!label _label_3
          (:`Exit`
            (`ActorComponent.Deactivate` (`self.ParticleSystem2`))
            (`SceneComponent.SetVisibility` (`self.MissingPipeCurveSection`) true true)
            (`|ExecutionSequence`
              (:`then_0`
                (goto _label :!via `Close`))
              (:`then_1`
                (goto _label_2))
              (:`then_2`
                _)))))
      (:`then_1`
        ;[1 1 1] Handles Alll The Input For The X Section
        (`/Engine/EditorBlueprintResources/StandardMacros.Gate` true :!label _label_4
          (:`Exit`
            (`ActorComponent.Deactivate` (`self.ParticleSystem1`))
            (`ActorComponent.Deactivate` (`self.ParticleSystem6`))
            (`ActorComponent.Deactivate` (`self.ParticleSystem7`))
            (`SceneComponent.SetVisibility` (`self.MissingPipeXSection1`) true true)
            (`|ExecutionSequence`
              (:`then_0`
                (goto _label_8 :!via `Close`))
              (:`then_1`
                (bind _outactors (`GameplayStatics.GetAllActorsOfClass` "/Game/PlayerController/Gat_PlayerHUD.Gat_PlayerHUD_C" :!label _label_5))
                (message `/Game/Meshes/Props/Pipes/BPI_PipeInterface.PipeToHudOutVolume` _outactors)
                (`self.DisableInput` _returnvalue_2)
                (goto _label_4 :!via `Close`))
              (:`then_2`
                _)))))
      (:`then_2`
        ;[1 1 1] Handles All the Input For The T Section
        (`/Engine/EditorBlueprintResources/StandardMacros.Gate` true :!label _label_6
          (:`Exit`
            (`ActorComponent.Deactivate` (`self.ParticleSystem3`))
            (`ActorComponent.Deactivate` (`self.ParticleSystem4`))
            (`ActorComponent.Deactivate` (`self.ParticleSystem5`))
            (`SceneComponent.SetVisibility` (`self.MissingPipeTSection`) true true)
            (`|ExecutionSequence`
              (:`then_0`
                (goto _label_9 :!via `Close`))
              (:`then_1`
                (bind _outactors_2 (`GameplayStatics.GetAllActorsOfClass` "/Game/PlayerController/Gat_PlayerHUD.Gat_PlayerHUD_C" :!label _label_7))
                (message `/Game/Meshes/Props/Pipes/BPI_PipeInterface.PipeToHudOutVolume` _outactors_2)
                (`self.DisableInput` _returnvalue)
                (goto _label_6 :!via `Close`))
              (:`then_2`
                _))))))
    ;[1 1 1] Passes A Bool To The Access Panel
    (`|MultiGate` false
      (:`Out 0`
        (`AudioComponent.FadeOut` (`self.Audio1`) 0.0 0.0))
      (:`Out 1`
        (`AudioComponent.FadeOut` (`self.Audio2`) 0.0 0.0))
      (:`Out 2`
        (set `/Game/Meshes/Props/AccessPanel/BP_DoorAcessPanelVisual.bObjectiveCompleted` true (`self.AccessPanel`))
        (`AudioComponent.FadeOut` (`self.Audio3`) 0.0 0.0)))))

(event `self.XSectionTrigger.OnComponentBeginOverlap`
  (params (OtherActor :type "Actor Object Reference") (OtherComp :type "PrimitiveComponent Object Reference") (OtherBodyIndex :type Integer) (bFromSweep :type Boolean) (SweepResult :type "EngineTypes.HitResult Structure (by ref)"))
  ;[1 1 1] Handles Alll The Input For The X Section
  (if (`/Game/Meshes/Props/Pipes/BP_GAT_Pipe_XSection.bCollected` (`self.PickupXSection`))
    (`/Engine/EditorBlueprintResources/StandardMacros.Gate` false :!label _label_8
      (:`Exit`
        (bind _outactors (`GameplayStatics.GetAllActorsOfClass` "/Game/PlayerController/Gat_PlayerHUD.Gat_PlayerHUD_C"))
        (message `/Game/Meshes/Props/Pipes/BPI_PipeInterface.Pipe To HUD In Volume` _outactors)
        (`self.EnableInput` (`GameplayStatics.GetPlayerController` 0))
        (goto _label_4 :!via `Open`)))))

(event `self.TSectionTrigger.OnComponentBeginOverlap`
  (params (OtherActor :type "Actor Object Reference") (OtherComp :type "PrimitiveComponent Object Reference") (OtherBodyIndex :type Integer) (bFromSweep :type Boolean) (SweepResult :type "EngineTypes.HitResult Structure (by ref)"))
  ;[1 1 1] Handles All the Input For The T Section
  (if (`/Game/Meshes/Props/Pipes/BP_GAT_MissingPipeTSection.bCollected` (`self.PickupTSection`))
    (`/Engine/EditorBlueprintResources/StandardMacros.Gate` false :!label _label_9
      (:`Exit`
        (bind _outactors (`GameplayStatics.GetAllActorsOfClass` "/Game/PlayerController/Gat_PlayerHUD.Gat_PlayerHUD_C"))
        (message `/Game/Meshes/Props/Pipes/BPI_PipeInterface.Pipe To HUD In Volume` _outactors)
        (`self.EnableInput` (`GameplayStatics.GetPlayerController` 0))
        (goto _label_6 :!via `Open`)))))

(event `self.XSectionTrigger.OnComponentEndOverlap`
  (params (OtherActor :type "Actor Object Reference") (OtherComp :type "PrimitiveComponent Object Reference") (OtherBodyIndex :type Integer))
  ;[1 1 1] Handles Alll The Input For The X Section
  (goto _label_5))

(event `self.TSectionTrigger.OnComponentEndOverlap`
  (params (OtherActor :type "Actor Object Reference") (OtherComp :type "PrimitiveComponent Object Reference") (OtherBodyIndex :type Integer))
  ;[1 1 1] Handles All the Input For The T Section
  (goto _label_7))

(fn `UserConstructionScript`
  (`SceneComponent.SetVisibility` (`self.MissingPipeXSection1`) false true)
  (`SceneComponent.SetVisibility` (`self.MissingPipeTSection`) false true)
  (`SceneComponent.SetVisibility` (`self.MissingPipeCurveSection`) false true))