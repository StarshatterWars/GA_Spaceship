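; Pipe prop that explodes once when anything overlaps its trigger, swapping to a damaged mesh with fire.
; A gate limits it to one blast, which randomly scales both effects, plays sound and restarts the explosion particles through a delayed DoN loop.
; The player takes equal damage at any distance, with a hurt sound mix only up close.
; The fire's X offset uses fresh random rolls rather than its actual scale.
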(event `self.ExplosionTrigger.OnComponentBeginOverlap`
  (params (OtherActor :type "Actor Object Reference") (OtherComp :type "PrimitiveComponent Object Reference") (OtherBodyIndex :type Integer) (bFromSweep :type Boolean) (SweepResult :type "EngineTypes.HitResult Structure (by ref)"))
  (bind _returnvalue (`KismetMathLibrary.RandomFloatInRange` 1.0 4.0))
  (bind _returnvalue_2 (`GameplayStatics.GetPlayerCharacter` 0))
  (bind _explosion (`self.Explosion`))
  (bind _fire (`self.Fire`))
  (bind _returnvalue_3 (`self.GetDistanceTo` _returnvalue_2 self))
  (bind _x (.x (`SceneComponent.RelativeLocation` _fire)))
  (bind _y (.y (`SceneComponent.RelativeLocation` _fire)))
  (bind _z (.z (`SceneComponent.RelativeLocation` _fire)))
  ;[1 1 1] Only One Explosion Per Pipe
  (`/Engine/EditorBlueprintResources/StandardMacros.Gate` false :!label _label
    (:`Exit`
      (`|ExecutionSequence`
        (:`then_0`
          ;[1 1 1] Sets A Random Scale Value For Particle Effects
          (`SceneComponent.SetRelativeScale3D` _explosion (`KismetMathLibrary.MakeVector` (`KismetMathLibrary.RandomFloatInRange` 1.0 2.0) (`KismetMathLibrary.RandomFloatInRange` 1.0 2.0) (`KismetMathLibrary.RandomFloatInRange` 1.0 2.0)))
          (`SceneComponent.SetRelativeScale3D` (`self.Fire`) (`KismetMathLibrary.MakeVector` _returnvalue (`KismetMathLibrary.RandomFloatInRange` 1.0 4.0) (`KismetMathLibrary.RandomFloatInRange` 1.0 4.0)))
          ;[1 1 1] Triggers First Explosion
          (`ActorComponent.Deactivate` _explosion)
          (`SceneComponent.SetVisibility` _explosion true false)
          (`ActorComponent.Activate` _explosion false)
          (`GameplayStatics.PlaySoundAttached` "/Game/Audio/SFX/Explosion_Cue.Explosion_Cue" (`self.K2_GetRootComponent`))
          (`|ExecutionSequence`
            (:`then_0`
              ;[1 1 1] Triggers The Explosion Again For Good Measure
              (`|ExecutionSequence` :!label _label_2
                (:`then_0`
                  (`/Engine/EditorBlueprintResources/StandardMacros.Do N` 2
                    (:`Exit`
                      (`ActorComponent.Deactivate` _explosion))))
                (:`then_1`
                  (`KismetSystemLibrary.Delay` 0.5)
                  (goto _label_2))
                (:`then_2`
                  (`/Engine/EditorBlueprintResources/StandardMacros.Do N` 1
                    (:`Exit`
                      (`ActorComponent.Activate` _explosion false))))))
            (:`then_1`
              ;[1 1 1] Switches The Pipe Mesh And Fire Effect
              (`KismetSystemLibrary.Delay` 0.1)
              (`SceneComponent.SetVisibility` (`self.PostExplosion`) true false)
              (`SceneComponent.SetVisibility` (`self.PreExplosion`) false false)
              (`SceneComponent.SetVisibility` (`self.Fire`) true false))
            (:`then_2`
              ;[1 1 1] Applys Damage To The Player Character
              (if (<= _returnvalue_3 100.0)
                (`GameplayStatics.ApplyDamage` _returnvalue_2 40.0 null self)
                (`GameplayStatics.PushSoundMixModifier` "/Game/Audio/SoundClassAndMixes/Hurt_EQ.Hurt_EQ")
                (`KismetSystemLibrary.PrintString` "Hello")
                (elif (<= _returnvalue_3 200.0)
                  (`GameplayStatics.ApplyDamage` _returnvalue_2 40.0 null self)
                  (elif (<= _returnvalue_3 300.0)
                    (`GameplayStatics.ApplyDamage` _returnvalue_2 40.0 null self)
                    (else
                      (`GameplayStatics.ApplyDamage` _returnvalue_2 40.0 null self))))))
            (:`then_3`
              ;[1 1 1] Checks The Scale Of The Fire In The X-Axis And adjusts The Location To Accomodate
              (if (`KismetMathLibrary.NearlyEqual_FloatFloat` _returnvalue 1.0 0.2)
                _
                (elif (`KismetMathLibrary.NearlyEqual_FloatFloat` _returnvalue 2.0 0.2)
                  (`SceneComponent.K2_SetRelativeLocation` _fire (`KismetMathLibrary.MakeVector` (+ (* _returnvalue 2.0) _x) _y _z) false)
                  (else
                    (`SceneComponent.K2_SetRelativeLocation` _fire (`KismetMathLibrary.MakeVector` (+ (* _returnvalue 4.0) _x) _y _z) false)))))))
        (:`then_1`
          (goto _label :!via `Close`))))))

(fn `UserConstructionScript`
  (`SceneComponent.SetVisibility` (`self.PostExplosion`) false false)
  (`SceneComponent.SetVisibility` (`self.Explosion`) false false)
  (`SceneComponent.SetVisibility` (`self.Fire`) false false)
  (`ActorComponent.Deactivate` (`self.Explosion`)))