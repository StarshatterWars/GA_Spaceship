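; Proximity mine that explodes when a Player-tagged actor touches its inner trigger, or when a countdown runs out.
; Entering the outer trigger starts audio and a one-second Gate/Delay countdown loop; leaving stops both and resets the count.
; Detonation spawns an explosion effect, removes the mine component, then applies radial falloff damage after a short delay and destroys the actor.
; The outer trigger does not filter by actor.
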(event `self.InnerTrigger.OnComponentBeginOverlap`
  (params (OverlappedComponent :type "PrimitiveComponent Object Reference") (OtherActor :type "Actor Object Reference") (OtherComp :type "PrimitiveComponent Object Reference") (OtherBodyIndex :type Integer) (bFromSweep :type Boolean) (SweepResult :type "HitResult Structure (by ref)"))
  (bind _mine (`self.Mine`))
  (bind _secondsleft (`self.SecondsLeft`))
  ;[1 1 1] Trigger To Cause Immiediate Explosion
  (if (`self.ActorHasTag` OtherActor "Player")
    (`|ExecutionSequence`
      (:`then_0`
        ;[1 1 1] Creates Particle Effect And Damages The Player
        (`|SpawnActorFromClass` "/Game/Blueprints/Blueprint_Effect_Explosion.Blueprint_Effect_Explosion_C" (`SceneComponent.K2_GetComponentToWorld` (`self.InnerTrigger`)) "AdjustIfPossibleButDontSpawnIfColliding" "OverrideRootScale" :!label _label)
        (`|ExecutionSequence`
          (:`then_0`
            (`KismetSystemLibrary.Delay` 0.3)
            (`GameplayStatics.ApplyRadialDamageWithFalloff` 20.0 5.0 (`self.K2_GetActorLocation`) 50.0 500.0 0.1)
            (`self.K2_DestroyActor`))
          (:`then_1`
            (`/Engine/EditorBlueprintResources/StandardMacros.IsValid` _mine
              (:`Is Valid`
                (`ActorComponent.K2_DestroyComponent` _mine))))))
      (:`then_1`
        (goto _label_4 :!via `Close`)))))

(event `self.OuterTrigger.OnComponentEndOverlap`
  (params (OverlappedComponent :type "PrimitiveComponent Object Reference") (OtherActor :type "Actor Object Reference") (OtherComp :type "PrimitiveComponent Object Reference") (OtherBodyIndex :type Integer))
  (bind _secondsleft (`self.SecondsLeft`))
  (bind _audio1 (`self.Audio1`))
  (`|ExecutionSequence`
    (:`then_0`
      ;[1 1 1] Logic To Explode The Mine After Ten Seconds If Player Does Not Move Out Of Blast Radius
      (set `self.SecondsLeft` 5)
      (`AudioComponent.FadeOut` _audio1 0.2 0.0))
    (:`then_1`
      (goto _label_4 :!via `Close`))
    (:`then_2`
      (goto _label_2 :!via `Reset`))))

(event `self.OuterTrigger.OnComponentBeginOverlap`
  (params (OverlappedComponent :type "PrimitiveComponent Object Reference") (OtherActor :type "Actor Object Reference") (OtherComp :type "PrimitiveComponent Object Reference") (OtherBodyIndex :type Integer) (bFromSweep :type Boolean) (SweepResult :type "HitResult Structure (by ref)"))
  (bind _secondsleft (`self.SecondsLeft`))
  (`/Engine/EditorBlueprintResources/StandardMacros.DoOnce` false :!label _label_2
    (:`Completed`
      (`|ExecutionSequence`
        (:`then_0`
          (goto _label_4 :!via `Open`))
        (:`then_1`
          ;[1 1 1] Logic To Explode The Mine After Ten Seconds If Player Does Not Move Out Of Blast Radius
          (`|ExecutionSequence` :!label _label_3
            (:`then_0`
              (`/Engine/EditorBlueprintResources/StandardMacros.Gate` false :!label _label_4
                (:`Exit`
                  (`KismetSystemLibrary.Delay` 1.0)
                  (goto _label_3))))
            (:`then_1`
              (if (== _secondsleft 0)
                (goto _label)
                (else
                  (set `self.SecondsLeft` (- _secondsleft 1)))))))
        (:`then_2`
          (`AudioComponent.Play` (`self.Audio1`) 0.0))))))

(fn `UserConstructionScript`)