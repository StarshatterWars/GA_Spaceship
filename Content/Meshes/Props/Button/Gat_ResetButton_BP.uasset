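; Reset button prop that animates a push on interact and broadcasts reset interact and release events.
; A timeline slides the Button mesh along X and reverses via a MultiGate when finished, with a Gate that closes afterwards and reopens on release.
; OnInteract also loops over all handle, button and dial actors, but only casts them without calling anything on them.
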(event `self.OnInteract`
  ;[1 1 1] Animates The Button When The Player Interacts With The Object
  (`|ExecutionSequence`
    (:`then_0`
      (`/Engine/EditorBlueprintResources/StandardMacros.Gate` false :!label _label
        (:`Exit`
          (bind (_direction _push) (`Timeline|Timeline_0` :!label _label_2)
            (:`Update`
              (`SceneComponent.K2_SetRelativeLocation` (`self.Button`) (`KismetMathLibrary.MakeVector` _push 0.0 0.0) false))
            (:`Finished`
              (`|MultiGate` false true
                (:`Out 0`
                  (`|ExecutionSequence`
                    (:`then_0`
                      (goto _label_2 :!via `Reverse`))
                    (:`then_1`
                      (goto _label :!via `Close`))))))))))
    (:`then_1`
      ;[1 1 1] Casts A Reset Signal To Each Of The Pulleys
      (bind _outactors (`GameplayStatics.GetAllActorsOfClass` "/Game/Meshes/Props/HandleLever/Gat_Handle_BP.Gat_Handle_BP_C"))
      (for _array_element _outactors
        (cast `/Game/Meshes/Props/HandleLever/Gat_Handle_BP` _array_element)))
    (:`then_2`
      (bind _outactors_2 (`GameplayStatics.GetAllActorsOfClass` "/Game/Meshes/Props/Button/Gat_Button_BP.Gat_Button_BP_C"))
      (for _array_element_2 _outactors_2
        (cast `/Game/Meshes/Props/Button/Gat_Button_BP` _array_element_2)))
    (:`then_3`
      (bind _outactors_3 (`GameplayStatics.GetAllActorsOfClass` "/Game/Meshes/Props/Dial/Gat_Dial_BP.Gat_Dial_BP_C"))
      (for _array_element_3 _outactors_3
        (cast `/Game/Meshes/Props/Dial/Gat_Dial_BP` _array_element_3)))
    (:`then_4`
      (`self.ResetInteract`))))

(event `self.OnRelease`
  ;[1 1 1] Animates The Button When The Player Interacts With The Object
  (`|ExecutionSequence`
    (:`then_0`
      (goto _label :!via `Open`))
    (:`then_1`
      (`self.ResetRelease`))))

(fn `UserConstructionScript`)