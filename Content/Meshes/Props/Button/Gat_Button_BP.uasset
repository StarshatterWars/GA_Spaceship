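; Interactable push button prop that animates when pressed and signals its interact and release to other logic.
; On interact, the ButtonPush timeline slides the Button component along its relative X axis, and ButtonInteract is called.
; Release or actor end overlap reverses the timeline and calls ButtonRelease.
; Two DoOnce gates re-arm each other, so presses and releases alternate without repeating.
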(event `self.OnInteract`
  ;[1 1 1] Animates The Button When The Player Interacts With The Object
  (`/Engine/EditorBlueprintResources/StandardMacros.DoOnce` false :!label _label
    (:`Completed`
      (`|ExecutionSequence`
        (:`then_0`
          (bind (_direction _push) (`Timeline|ButtonPush` :!label _label_2)
            (:`Update`
              (`SceneComponent.K2_SetRelativeLocation` (`self.Button`) (`KismetMathLibrary.MakeVector` _push 12.0 -14.0) false))))
        (:`then_1`
          (`self.ButtonInteract`))
        (:`then_2`
          (goto _label_3 :!via `Reset`))))))

(event `self.OnRelease`
  ;[1 1 1] Animates The Button When The Player Interacts With The Object
  (`/Engine/EditorBlueprintResources/StandardMacros.DoOnce` false :!label _label_3
    (:`Completed`
      (`|ExecutionSequence`
        (:`then_0`
          (goto _label_2 :!via `Reverse`))
        (:`then_1`
          (`self.ButtonRelease`))
        (:`then_2`
          (goto _label :!via `Reset`))))))

(event `self.ReceiveActorEndOverlap`
  (params (OtherActor :type "Actor Object Reference"))
  ;[1 1 1] Animates The Button When The Player Interacts With The Object
  (goto _label_3))

(fn `UserConstructionScript`)